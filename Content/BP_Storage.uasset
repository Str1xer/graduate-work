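; BP_Storage is a storage actor that holds a running count of resources and shows it on a text render component.
; BeginPlay writes the starting count to the text.
; The AddResource event adds the given amount to the count and refreshes the displayed number.
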(event `self.ReceiveBeginPlay`
  (`TextRenderComponent.K2_SetText` (`self.TextRender`) (`KismetTextLibrary.Conv_IntToText` (`self.CountOfResources`))))

(event `self.AddResource`
  (params (count :type Integer))
  (bind _output_get (set `self.CountOfResources` (+ count (`self.CountOfResources`))))
  (`TextRenderComponent.K2_SetText` (`self.TextRender`) (`KismetTextLibrary.Conv_IntToText` _output_get)))

(fn `UserConstructionScript`)