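; Enemy actor Blueprint that computes per-foot ground placement data on every tick, consistent with foot IK.
; Downward visibility traces under each ankle socket find the ground near the actor's base.
; Each hit yields a foot offset relative to a point below the actor's origin, plus a roll and pitch rotation aligned to the surface normal.
; Results are stored in left and right variables, with no other gameplay logic.
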(event `self.ReceiveTick`
  (params (DeltaSeconds :type "Float (single-precision)"))
  (bind _z (.z (`self.K2_GetActorLocation`)))
  (bind _returnvalue_location (`KismetMathLibrary.BreakTransform` (`SceneComponent.GetSocketTransform` (`self.Mesh`) "r_ankle1" "RTS_World")))
  (bind (_returnvalue_location_2 _returnvalue_rotation) (`KismetMathLibrary.BreakTransform` (`SceneComponent.GetSocketTransform` (`self.Mesh`) "r_ankle1" "RTS_World")))
  (bind _z_2 (.z (`self.K2_GetActorLocation`)))
  (bind _returnvalue_location_3 (`KismetMathLibrary.BreakTransform` (`SceneComponent.GetSocketTransform` (`self.Mesh`) "l_ankle1" "RTS_World")))
  (bind (_returnvalue_location_4 _returnvalue_rotation_2) (`KismetMathLibrary.BreakTransform` (`SceneComponent.GetSocketTransform` (`self.Mesh`) "l_ankle1" "RTS_World")))
  (bind _returnvalue (`KismetMathLibrary.GetUpVector` _returnvalue_rotation_2))
  (bind _x (.x _returnvalue_location))
  (bind _y (.y _returnvalue_location))
  (bind _x_2 (.x _returnvalue_location_3))
  (bind _y_2 (.y _returnvalue_location_3))
  (bind _returnvalue_2 (`KismetMathLibrary.GetUpVector` _returnvalue_rotation))
  (bind _outhit (`KismetSystemLibrary.LineTraceSingle` (`KismetMathLibrary.MakeVector` _x_2 _y_2 (- _z_2 65.0)) (`KismetMathLibrary.MakeVector` _x_2 _y_2 (- _z_2 130.0)) "TraceTypeQuery1"))
  (bind (_bblockinghit _binitialoverlap _time _distance _location _impactpoint _normal _impactnormal) (`GameplayStatics.BreakHitResult` _outhit))
  (set `self.Left_Offset` (- _impactpoint (- (`self.K2_GetActorLocation`) (0.0 0.0 88.0))))
  (bind (_returnvalue_roll _returnvalue_pitch) (`KismetMathLibrary.BreakRotator` (`KismetMathLibrary.MakeRotFromZX` _impactnormal (`KismetMathLibrary.RotateAngleAxis` (`KismetMathLibrary.GetForwardVector` _returnvalue_rotation_2) (* (`KismetMathLibrary.DegAcos` (`KismetMathLibrary.Dot_VectorVector` _impactnormal _returnvalue)) 1.0) (`KismetMathLibrary.Normal` (`KismetMathLibrary.Cross_VectorVector` _impactnormal _returnvalue))))))
  (set `self.LeftRotation` (`KismetMathLibrary.MakeRotator` _returnvalue_roll _returnvalue_pitch))
  (bind _outhit_2 (`KismetSystemLibrary.LineTraceSingle` (`KismetMathLibrary.MakeVector` _x _y (- _z 65.0)) (`KismetMathLibrary.MakeVector` _x _y (- _z 130.0)) "TraceTypeQuery1"))
  (bind (_bblockinghit_2 _binitialoverlap_2 _time_2 _distance_2 _location_2 _impactpoint_2 _normal_2 _impactnormal_2) (`GameplayStatics.BreakHitResult` _outhit_2))
  (set `self.Right_Offset` (- _impactpoint_2 (- (`self.K2_GetActorLocation`) (0.0 0.0 88.0))))
  (bind (_returnvalue_roll_2 _returnvalue_pitch_2) (`KismetMathLibrary.BreakRotator` (`KismetMathLibrary.MakeRotFromZX` _impactnormal_2 (`KismetMathLibrary.RotateAngleAxis` (`KismetMathLibrary.GetForwardVector` _returnvalue_rotation) (* (`KismetMathLibrary.DegAcos` (`KismetMathLibrary.Dot_VectorVector` _impactnormal_2 _returnvalue_2)) -1.0) (`KismetMathLibrary.Normal` (`KismetMathLibrary.Cross_VectorVector` _impactnormal_2 _returnvalue_2))))))
  (set `self.RightRotation` (`KismetMathLibrary.MakeRotator` _returnvalue_roll_2 _returnvalue_pitch_2)))

(fn `UserConstructionScript`)